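; BP_Gun is an automatic gun that fires BP_Bullet projectiles for the player character when it has a rifle.
; It binds to the character's shoot start/stop events; ShootCall re-arms a timer at FireRate until stopped.
; Bullets spawn at the muzzle socket using the character's root rotation, with random yaw spread when not aiming down sights.
; Emitter and sound nodes are present but unconnected.
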(event Custom|ShootCall
  (if (Variables|Default|GetCanShoot?)
    (if (Variables|/Game/ThirdPerson/Blueprints/BP_MainCharacter.BP_MainCharacter_C|GetADS (Variables|Default|GetBP_MainChacterREF))
      ;[1 1 1] LineTrace
      (CallFunction|ADSShoot)
      (else
        (CallFunction|NonADS)))
    (bind _returnvalue (Utilities|Time|SetTimerbyEvent (delegate Custom|ShootCall) (/ 1.0 (Variables|Default|GetFireRate))))
    (Variables|Default|SetGunTimerREF _returnvalue)))

(event Custom|StopShoot
  (Utilities|Time|ClearandInvalidateTimerbyHandle (Variables|Default|GetGunTimerREF)))

(event EventBeginPlay
  (bind _asbp_main_character (Utilities|Casting|CastToBP_MainCharacter (Game|Player|GetPlayerPawn 0)))
  (bind _output_get (Variables|Default|SetBP_MainChacterREF _asbp_main_character))
  (EventDispatchers|BindEventtoShootStart _output_get (EventDispatchers|CreateEvent :!event Custom|ShootCall))
  (EventDispatchers|BindEventtoShootStop _output_get (EventDispatchers|CreateEvent :!event Custom|StopShoot)))

(event EventTick
  (params (DeltaSeconds :type Float%20%28single-precision%29))
  (Variables|Default|SetCanShoot? (Variables|/Game/ThirdPerson/Blueprints/BP_MainCharacter.BP_MainCharacter_C|GetHasRifle? (Variables|Default|GetBP_MainChacterREF))))

(fn ConstructionScript)

(fn ADSShoot
  ;[1 0 0] Projectile
  (Game|SpawnActorfromClass "/Game/Gun/Blueprints/BP_Bullet.BP_Bullet_C" (Math|Transform|MakeTransform (Transformation|GetSocketLocation (Variables|Default|GetGun) "Projectile_Socket") (Transformation|GetWorldRotation (Variables|/Script/Engine.Actor|GetRootComponent (Variables|Default|GetBP_MainChacterREF)))) "Undefined" 0 0))

(fn NonADS
  (bind _bp_mainchacterref (Variables|Default|GetBP_MainChacterREF))
  (bind _gunspread (Variables|Default|GetGunSpread))
  (bind _rootcomponent (Variables|/Script/Engine.Actor|GetRootComponent _bp_mainchacterref))
  (bind _returnvalue (Transformation|GetWorldRotation _rootcomponent))
  (bind (_roll _pitch _yaw) (Math|Rotator|BreakRotator _returnvalue))
  ;[1 0 0] Projectile
  (Game|SpawnActorfromClass "/Game/Gun/Blueprints/BP_Bullet.BP_Bullet_C" (Math|Transform|MakeTransform (Transformation|GetSocketLocation (Variables|Default|GetGun) "Projectile_Socket") (Math|Rotator|MakeRotator _roll _pitch (+ _yaw (Math|Random|RandomFloatinRange (* _gunspread -1.0) _gunspread)))) "Undefined" 0 0))